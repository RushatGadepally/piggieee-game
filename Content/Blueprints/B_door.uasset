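; B_door is a door Blueprint that opens when enough linked switches are active.
; Switch activation and deactivation events raise or lower a counter, which is compared against the required switch count.
; Meeting the count plays the Activation timeline, which moves the Door component's relative Z; otherwise the timeline reverses.
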(event Custom|Switch_Activated
  (Math|Integer|IncrementInt (Variables|Default|Getpress_swithact)
    (:%20%20
      (if (>= (Variables|Default|Getpress_swithact) (Variables|Default|Getpress_swithneed))
        (bind _newtrack_3 (Timeline|activation Play)
          (:Update
            (Transformation|SetRelativeLocation (Variables|Default|Getdoor) (Math|Vector|MakeVector 0.0 0.0 _newtrack_3) false false)))
        (else
          (Timeline|activation Reverse))))))

(event Custom|Switch_Decativated
  (Math|Integer|DecrementInt (Variables|Default|Getpress_swithact)
    (:%20%20
      (if (>= (Variables|Default|Getpress_swithact) (Variables|Default|Getpress_swithneed))
        (bind _newtrack_3 (Timeline|activation Play)
          (:Update
            (Transformation|SetRelativeLocation (Variables|Default|Getdoor) (Math|Vector|MakeVector 0.0 0.0 _newtrack_3) false false)))
        (else
          (Timeline|activation Reverse))))))

(event EventBeginPlay)

(event Collision|EventActorBeginOverlap
  (params (OtherActor :type Actor%20Object%20Reference)))

(event EventTick
  (params (DeltaSeconds :type Float%20%28single-precision%29)))

(fn ConstructionScript)